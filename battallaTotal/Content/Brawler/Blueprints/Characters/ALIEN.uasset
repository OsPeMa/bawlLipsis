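; Alien character Blueprint for the Brawler game, a child class that specializes the material setup of its parent character.
; BeginPlay runs the parent logic, then calls the overridden CreateMaterial.
; That override calls the parent version, then sets the mesh's first material slot from an alien skins array indexed by SkinIndex.
; Dynamic material instance nodes in that function are unconnected and never run.
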(event EventBeginPlay
  (|CallParentFunction)
  (CallFunction|CreateMaterial))

(event Collision|EventActorBeginOverlap
  (params (OtherActor :type Actor%20Object%20Reference)))

(event EventTick
  (params (DeltaSeconds :type Float%20%28single-precision%29))
  (|CallParentFunction DeltaSeconds) ; This node is disabled and will not be called.\nDrag off pins to build functionality.
)

(fn ConstructionScript
  (|CallParentFunction))

(fn CreateMaterial
  (|CallParentFunction)
  (Rendering|Material|SetMaterial (Variables|Character|GetMesh) 0 (Utilities|Array|Get(acopy) (Utilities|Struct|BreakAlienSkins (Utilities|Struct|MakeAlienSkins "\"/Game/Resources/Meshes/alienPelea/Alien/Aline_MAT.Aline_MAT\"',Material'\"/Game/Resources/Meshes/alienPelea/Alien/AlienTXT/Alien_RidleySkin_Mat.Alien_RidleySkin_Mat\"")) (Variables|Default|GetskinIndex))))