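; Game mode for the brawler's character selection screen, tracking who joins and which skin they pick.
; BeginPlay initializes the BrawlKey on the SpaceInstance game instance, then creates local players by matching PlayerStart tags to indices.
; Registering, kicking and skin changes update that key's player list and activate, deactivate or re-skin the matching cage.
; Cages are registered by index in the Jaulas map through AddCage.
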(event EventBeginPlay
  (bind _asspace_instance (Utilities|Casting|CastToSpaceInstance (Game|GetGameInstance)))
  (bind _output_get (Variables|Default|SetAs%20Space%20Instance _asspace_instance))
  (Variables|/Game/Resources/Utilites/SpaceInstance.SpaceInstance_C|SetBrawlKey _output_get (Utilities|Struct|MakeStartBrawlerGameKey (Variables|Default|GetPlayer%20List)))
  (bind _outactors (Actor|GetAllActorsOfClass "/Script/Engine.PlayerStart"))
  (bind _output_get_2 (Variables|Default|SetPlayerStartArray _outactors))
  (for _index (range 0 (Utilities|Array|Length _output_get_2))
    (Variables|Default|SetIndex _index)
    (for _array_element (Variables|Default|GetPlayerStartArray)
      (if (Utilities|Name|Equal(Name) (Variables|/Script/Engine.PlayerStart|GetPlayerStartTag _array_element) (Utilities|String|StringToName (Utilities|String|ToString(Integer) (Variables|Default|GetIndex))))
        (Class|GameplayStatics|CreatePlayer (Variables|Default|GetIndex))))))

(event EventTick
  (params (DeltaSeconds :type Float%20%28single-precision%29)))

(fn ConstructionScript)

(fn RegisterPlayer
  (params (controlIndex :type Integer))
  (bind _activecharacters (Variables|Default|GetActiveCharacters))
  (bind _activecharacters_2 (Variables|Default|GetActiveCharacters))
  (bind _returnvalue (Utilities|Array|Add (Utilities|Struct|BreakStartBrawlerGameKey (Variables|/Game/Resources/Utilites/SpaceInstance.SpaceInstance_C|GetBrawlKey (Variables|Default|GetAs%20Space%20Instance))) (Utilities|Struct|MakePlayerCharacteristics _activecharacters controlIndex)))
  (Default|Active (.Value (Utilities|Map|Find (Variables|Default|GetJaulas) _activecharacters)))
  (Math|Integer|IncrementInt _activecharacters_2
    (:%20%20
      (return _returnvalue (- _activecharacters_2 1)))))

(fn KickPlayer
  (params (PlayerListIndex :type Integer) (CageIndex :type Integer))
  (Utilities|Array|RemoveIndex (Utilities|Struct|BreakStartBrawlerGameKey (Variables|/Game/Resources/Utilites/SpaceInstance.SpaceInstance_C|GetBrawlKey (Variables|Default|GetAs%20Space%20Instance))) PlayerListIndex)
  (Math|Integer|DecrementInt (Variables|Default|GetActiveCharacters)
    (:%20%20
      (Default|DesActive (.Value (Utilities|Map|Find (Variables|Default|GetJaulas) CageIndex))))))

(fn ChangeSkin
  (params (SkinIndex :type Integer) (PlayerIndex :type Integer) (CageIndex :type Integer))
  (bind _as_space_instance (Variables|Default|GetAs%20Space%20Instance))
  (bind _brawlkey (Variables|/Game/Resources/Utilites/SpaceInstance.SpaceInstance_C|GetBrawlKey _as_space_instance))
  (bind _playerlist (Utilities|Struct|BreakStartBrawlerGameKey _brawlkey))
  (bind _output (Utilities|Array|Get(acopy) _playerlist PlayerIndex))
  (bind (_characterindex _controllerindex) (Utilities|Struct|BreakPlayerCharacteristics _output))
  (Default|AsignMaterial (.Value (Utilities|Map|Find (Variables|Default|GetJaulas) CageIndex)) 0 (Utilities|Select :Index SkinIndex :Option%200 "NewEnumerator0" :Option%201 "NewEnumerator1"))
  (Utilities|Struct|SetmembersinPlayerCharacteristics _output _characterindex _controllerindex SkinIndex)
  (return))

(fn AddCage
  (params (cageIndex :type Integer) (cage :type Character%20Cage%20Object%20Reference))
  (Utilities|Map|Add (Variables|Default|GetJaulas) cageIndex cage))

(fn GetGamemodeCharacterSelector
  (return self))