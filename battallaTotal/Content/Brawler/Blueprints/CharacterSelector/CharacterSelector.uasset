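; Per-player input handler for the character selection screen, letting a player join, leave and cycle skins.
; On BeginPlay it gets the selector game mode through a message call, then delegates registration, kicking and skin changes to it using stored player and cage indices.
; Paired DoOnce gates make Start and Cancel alternate between join and leave.
; Skin input works only while joined and wraps between two skins.
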(event EventBeginPlay
  (bind _chselectgm (Class|CharacterSelectorGamemodeInterface|GetGamemodeCharacterSelector(Message) (Game|GetGameMode)))
  (Variables|Default|SetCh%20Select%20GM _chselectgm))

(event EventTick
  (params (DeltaSeconds :type Float%20%28single-precision%29)))

(event Input|ActionEvents|InputActionStart
  (params (Key :type Key%20Structure :default "None"))
  (bind _ch_select_gm (Variables|Default|GetCh%20Select%20GM))
  (:Pressed
    (Utilities|FlowControl|DoOnce false
      (:Completed
        (bind (_playerlistindex _cageindex) (Default|RegisterPlayer _ch_select_gm (Class|GameplayStatics|GetPlayerControllerID)))
        (Variables|Default|SetCage%20Index _cageindex)
        (Variables|Default|SetPlayer%20List%20Index _playerlistindex)
        (Variables|Default|SetisActive true)
        (Utilities|FlowControl|DoOnce true) ; enters at Reset
      ))))

(event Input|ActionEvents|InputActionCancel
  (params (Key :type Key%20Structure :default "None"))
  (bind _ch_select_gm (Variables|Default|GetCh%20Select%20GM))
  (:Pressed
    (Utilities|FlowControl|DoOnce true
      (:Completed
        (Default|KickPlayer _ch_select_gm (Variables|Default|GetPlayer%20List%20Index) (Variables|Default|GetCage%20Index))
        (Variables|Default|SetisActive false)
        (Utilities|FlowControl|DoOnce false) ; enters at Reset
      ))))

(event Input|ActionEvents|InputActionNextSkin
  (params (Key :type Key%20Structure :default "None"))
  (bind _skin (Variables|Default|Getskin))
  (:Pressed
    (if (Variables|Default|GetisActive)
      (Math|Integer|IncrementInt _skin
        (:%20%20
          (Default|ChangeSkin (Variables|Default|GetCh%20Select%20GM) (Math|Integer|%(Integer) (Math|Integer|Absolute(Integer) _skin) 2) (Variables|Default|GetPlayer%20List%20Index) (Variables|Default|GetCage%20Index)))))))

(event Input|ActionEvents|InputActionPrevSkin
  (params (Key :type Key%20Structure :default "None"))
  (bind _skin (Variables|Default|Getskin))
  (:Pressed
    (if (Variables|Default|GetisActive)
      (Math|Integer|DecrementInt _skin
        (:%20%20
          (Default|ChangeSkin (Variables|Default|GetCh%20Select%20GM) (Math|Integer|%(Integer) (Math|Integer|Absolute(Integer) _skin) 2) (Variables|Default|GetPlayer%20List%20Index) (Variables|Default|GetCage%20Index)))))))

(fn ConstructionScript)