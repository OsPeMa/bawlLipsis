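; CharacterCage is a display cage actor for the Brawler character selector.
; On BeginPlay it registers itself by index with the game mode's selector interface and spawns an ALIEN character at its skeletal mesh's transform.
; Active records the controller index, marks the cage in use, lights the spotlight and swaps the glass material; DesActive reverts these visuals and the in-use flag.
; AsignMaterial applies the chosen skin to the spawned character and the cage's skeletal mesh.
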(event EventBeginPlay
  (bind _chselectgm (Class|CharacterSelectorGamemodeInterface|GetGamemodeCharacterSelector(Message) (Game|GetGameMode)))
  (Default|AddCage _chselectgm (Variables|Default|Getindex) self)
  (bind _returnvalue (Game|SpawnActorfromClass "/Game/Brawler/Blueprints/Characters/Figthers/ALIEN.ALIEN_C" (Transformation|GetWorldTransform (Variables|Default|GetSkeletalMesh)) "Undefined" 0 0))
  (Variables|Default|SetCharacter _returnvalue))

(event Collision|EventActorBeginOverlap
  (params (OtherActor :type Actor%20Object%20Reference)))

(event EventTick
  (params (DeltaSeconds :type Float%20%28single-precision%29)))

(fn ConstructionScript)

(fn AsignMaterial
  (params (Material :type Material%20Interface%20Object%20Reference) (Skin :type AlienSkinsEnum%20Enum :default "NewEnumerator0") (SkinIndex :type Integer))
  (Variables|Default|SetSkin%20Index SkinIndex)
  (Default|SetMaterial (Variables|Default|GetCharacter) SkinIndex)
  (Rendering|Material|SetMaterial (Variables|Default|GetSkeletalMesh) 0 (Utilities|Select :Index Skin :NewEnumerator0 "/Game/Resources/Meshes/alienPelea/Alien/Aline_MAT.Aline_MAT" :NewEnumerator1 "/Game/Resources/Meshes/alienPelea/Alien/Ridley/Alien_RidleySkin_Mat.Alien_RidleySkin_Mat")))

(fn Active
  (params (ContollerIndex :type Integer))
  (Variables|Default|SetContoller%20Index ContollerIndex)
  (Variables|Default|SetinUse true)
  (Rendering|Components|Light|SetIntensity (Variables|Default|GetSpotLight) 1e+04)
  (Rendering|Material|SetMaterial (Variables|Default|GetGlass) 0 "/Game/StarterContent/Materials/M_Glass.M_Glass"))

(fn DesActive
  (Variables|Default|SetinUse false)
  (Rendering|Material|SetMaterial (Variables|Default|GetGlass) 0 "/Game/Resources/Meshes/Jaula/VidrioMat.VidrioMat")
  (Rendering|Components|Light|SetIntensity (Variables|Default|GetSpotLight) 0.0))